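; Master enemy Blueprint: a melee opponent that can smoothly turn toward the player, toggles lock-on marker and HP widget, and destroys itself on death.
; Hand collisions start disabled; overlaps spawn impact effects, with DoOnce gates reset by attack events limiting damage to BP_Fighter.
; A successful parry with SpecialDamage at least EnemyHP triggers the enemy's Hit animation, yet the fighter still takes damage.
; DistanceToPlayer line-traces to measure range and flags targetability.
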(event `/Game/ActionMAin/Character/Enemy/Enemy_InterFace/BP_Enemy_Action.Enemy_Dead`
  ;[1 1 1] 死亡
  (`self.K2_DestroyActor`))

(event `/Game/ActionMAin/Character/Enemy/Enemy_InterFace/BP_Enemy_Action.AttackLiset_L`
  ;[1 1 1] 攻撃
  (goto _label :!via `Reset`))

(event `/Game/ActionMAin/Character/Enemy/Enemy_InterFace/BP_LockOnSystem.LockOn`
  ;[1 1 1] インターフェイス
  (`/Engine/EditorBlueprintResources/StandardMacros.FlipFlop`
    (:`A`
      (`SceneComponent.SetVisibility` (`self.HPWidget`) true false)
      (`SceneComponent.SetVisibility` (`self.LockOnSphere`) true false))
    (:`B`
      (`SceneComponent.SetVisibility` (`self.LockOnSphere`) false false)
      (`SceneComponent.SetVisibility` (`self.HPWidget`) false false))))

(event `self.L_Hand_Collision.OnComponentBeginOverlap`
  (params (OverlappedComponent :type "PrimitiveComponent Object Reference") (OtherActor :type "Actor Object Reference") (OtherComp :type "PrimitiveComponent Object Reference") (OtherBodyIndex :type Integer) (bFromSweep :type Boolean) (SweepResult :type "HitResult Structure (by ref)"))
  ;[1 1 1] 攻撃
  (if (!= OtherActor self)
    (`self.HitFX` (`self.L_Hand_Collision`))
    (`/Engine/EditorBlueprintResources/StandardMacros.DoOnce` false :!label _label
      (:`Completed`
        (bind _asbp_fighter (cast `/Game/ActionMAin/Character/Player/BP_Fighter` OtherActor))
        (if (`/Game/ActionMAin/Character/Player/BP_Fighter.ParySucsessTime` _asbp_fighter)
          (if (>= (`/Game/ActionMAin/Character/Player/BP_Fighter.SpecialDamage` _asbp_fighter) (`self.EnemyHP`))
            (bind _asmaster_enemy_anim_bp (cast `/Game/ActionMAin/Character/Enemy/EnemyAnimset/AnimSet/MasterEnemy_AnimBP` (`SkeletalMeshComponent.GetAnimInstance` (`self.Mesh`))))
            (`/Game/ActionMAin/Character/Enemy/EnemyAnimset/AnimSet/MasterEnemy_AnimBP.Hit` _asmaster_enemy_anim_bp)))
        (`GameplayStatics.ApplyDamage` OtherActor (`self.Enemy_Damege`) null self)))))

(event `self.ReceiveBeginPlay`
  ;[1 1 1] HP表示
  (bind _asenemy_hp (cast `/Game/ActionMAin/UI/EnemyHP` (`WidgetComponent.GetUserWidgetObject` (`self.HPWidget`))))
  (set `/Game/ActionMAin/UI/EnemyHP.EnemyHP` (`self.EnemyHP`) _asenemy_hp))

(event `self.ReceiveTick`
  (params (DeltaSeconds :type "Float (single-precision)"))
  ;[1 1 1] プレイヤーを観る
  (`|ExecutionSequence`
    (:`then_0`
      (set `self.Delta` DeltaSeconds)
      (if (`self.FascePlayer`)
        (`self.K2_SetActorRotation` (`KismetMathLibrary.RInterpTo` (`self.K2_GetActorRotation`) (`KismetMathLibrary.FindLookAtRotation` (`self.K2_GetActorLocation`) (`self.K2_GetActorLocation` (`GameplayStatics.GetPlayerCharacter` 0))) (`self.Delta`) 4.0))))))

(event `self.R_Hand_Collision.OnComponentEndOverlap`
  (params (OverlappedComponent :type "PrimitiveComponent Object Reference") (OtherActor :type "Actor Object Reference") (OtherComp :type "PrimitiveComponent Object Reference") (OtherBodyIndex :type Integer))
  ;[1 1 1] 攻撃
  (if (!= OtherActor self)
    (`self.HitFX` (`self.R_Hand_Collision`))
    (`/Engine/EditorBlueprintResources/StandardMacros.DoOnce` false :!label _label_2
      (:`Completed`
        (bind _asbp_fighter (cast `/Game/ActionMAin/Character/Player/BP_Fighter` OtherActor))
        (if (`/Game/ActionMAin/Character/Player/BP_Fighter.ParySucsessTime` _asbp_fighter)
          (if (>= (`/Game/ActionMAin/Character/Player/BP_Fighter.SpecialDamage` _asbp_fighter) (`self.EnemyHP`))
            (bind _asmaster_enemy_anim_bp (cast `/Game/ActionMAin/Character/Enemy/EnemyAnimset/AnimSet/MasterEnemy_AnimBP` (`SkeletalMeshComponent.GetAnimInstance` (`self.Mesh`))))
            (`/Game/ActionMAin/Character/Enemy/EnemyAnimset/AnimSet/MasterEnemy_AnimBP.Hit` _asmaster_enemy_anim_bp)))
        (`GameplayStatics.ApplyDamage` OtherActor (`self.Enemy_Damege`) null self)))))

(event `/Game/ActionMAin/Character/Enemy/Enemy_InterFace/BP_Enemy_Action.AttackLiset_R`
  ;[1 1 1] 攻撃
  (goto _label_2 :!via `Reset`))

(fn `DistanceToPlayer`
  (bind _outhit (`KismetSystemLibrary.LineTraceSingleForObjects` (`self.K2_GetActorLocation`) (`self.K2_GetActorLocation` (`GameplayStatics.GetPlayerPawn` 0)) (`|MakeArray` "ObjectTypeQuery3" :!type "EObjectTypeQuery Enum") false (`|MakeArray` self :!type "Actor Object Reference") "None" true (struct :`R` 1.0 :`A` 1.0) (struct :`G` 1.0 :`A` 1.0) 0.1))
  (set `self.PlyerToEnemyDistance` (`.Distance` (`GameplayStatics.BreakHitResult` _outhit)))
  (set `self.CanBeTarge?` true)
  (return))

(fn `UserConstructionScript`
  (`PrimitiveComponent.SetCollisionEnabled` (`self.R_Hand_Collision`) "NoCollision")
  (`PrimitiveComponent.SetCollisionEnabled` (`self.L_Hand_Collision`) "NoCollision"))