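; Enemy character Blueprint, apparently a child of a master enemy, that handles taking damage in combat.
; AnyDamage on a living enemy triggers a brief hit stop through CustomTimeDilation, flags player awareness, then updates HP and its widget.
; Lethal damage plays knockdown, launches the body upward, disables targeting and calls the attacking fighter's lock-on event if locked.
; A parallel stamina pool acts as poise, playing a hit reaction and refilling when depleted.
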(event `self.ReceiveAnyDamage`
  (params (Damage :type "Float (single-precision)") (DamageType :type "DamageType Object Reference") (InstigatedBy :type "Controller Object Reference") (DamageCauser :type "Actor Object Reference"))
  ;[1 1 1] ダメージ処理
  ;[1 1 1] 被ダメージ
  (set `self.TakeDamage` (`KismetMathLibrary.FTrunc` Damage))
  ;[1 1 1] 死体か？
  (if (not (`self.Death?`))
    ;[1 1 1] Hit Stop
    (set `self.CustomTimeDilation` 0.0)
    (`KismetSystemLibrary.Delay` 0.1)
    (set `self.CustomTimeDilation` 1.0)
    ;[1 1 1] プレイヤー気付く
    (set `self.FascePlayer` true)
    (`|ExecutionSequence`
      (:`then_0`
        ;[1 1 1] HPより攻撃が高いか？
        (if (<= (`self.EnemyHP`) (`self.TakeDamage`))
          (bind _asbp_fighter (cast `/Game/ActionMAin/Character/Player/BP_Fighter` DamageCauser)
            (:`then`
              (if (`/Game/ActionMAin/Character/Player/BP_Fighter.TargetLocked?` _asbp_fighter)
                (`/Game/ActionMAin/Character/Player/BP_Fighter.LockOnEvent` _asbp_fighter))
              (set `self.EnemyHP` 0))
            (:`CastFailed`
              _))
          (bind _asenemy_hp (cast `/Game/ActionMAin/UI/EnemyHP` (`WidgetComponent.GetUserWidgetObject` (`self.HPWidget`))))
          (set `/Game/ActionMAin/UI/EnemyHP.EnemyHP` (`self.EnemyHP`) _asenemy_hp)
          ;[1 1 1] 死亡処理
          (bind _asmaster_enemy_anim_bp (cast `/Game/ActionMAin/Character/Enemy/EnemyAnimset/AnimSet/MasterEnemy_AnimBP` (`SkeletalMeshComponent.GetAnimInstance` (`self.Mesh`))))
          (`/Game/ActionMAin/Character/Enemy/EnemyAnimset/AnimSet/MasterEnemy_AnimBP.KnockDown` _asmaster_enemy_anim_bp)
          (`self.LaunchCharacter` (0.0 0.0 1500.0))
          (set `self.FascePlayer` false)
          (set `self.Death?` true)
          (set `self.CanBeTarge?` false)
          (else
            ;[1 1 1] ダメージ計算
            (set `self.EnemyHP` (- (`self.EnemyHP`) (`self.TakeDamage`)))
            (bind _asenemy_hp_2 (cast `/Game/ActionMAin/UI/EnemyHP` (`WidgetComponent.GetUserWidgetObject` (`self.HPWidget`))))
            (set `/Game/ActionMAin/UI/EnemyHP.EnemyHP` (`self.EnemyHP`) _asenemy_hp_2))))
      (:`then_1`
        ;[1 1 1] スタミナ切れ
        (if (< (`self.StaminaPoint`) (`self.TakeDamage`))
          (set `self.StaminaPoint` 0)
          (set `self.EnemyHitCondition` "NewEnumerator0")
          (bind _asmaster_enemy_anim_bp_2 (cast `/Game/ActionMAin/Character/Enemy/EnemyAnimset/AnimSet/MasterEnemy_AnimBP` (`SkeletalMeshComponent.GetAnimInstance` (`self.Mesh`))))
          (`/Game/ActionMAin/Character/Enemy/EnemyAnimset/AnimSet/MasterEnemy_AnimBP.Hit` _asmaster_enemy_anim_bp_2)
          (set `self.EnemyHitCondition` "NewEnumerator2")
          (set `self.StaminaPoint` 800)
          (else
            ;[1 1 1] スタミナダメージ
            (set `self.StaminaPoint` (- (`self.StaminaPoint`) (`self.TakeDamage`)))
            (if (<= (`self.StaminaPoint`) 0)
              (set `self.StaminaPoint` 0)
              (set `self.EnemyHitCondition` "NewEnumerator0")
              (bind _asmaster_enemy_anim_bp_3 (cast `/Game/ActionMAin/Character/Enemy/EnemyAnimset/AnimSet/MasterEnemy_AnimBP` (`SkeletalMeshComponent.GetAnimInstance` (`self.Mesh`))))
              (`/Game/ActionMAin/Character/Enemy/EnemyAnimset/AnimSet/MasterEnemy_AnimBP.Hit` _asmaster_enemy_anim_bp_3)
              (set `self.EnemyHitCondition` "NewEnumerator2")
              (set `self.StaminaPoint` 800))))))))

(fn `UserConstructionScript`
  (`parent.UserConstructionScript`))